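; A platform that falls after the player character steps into its trigger, then returns to its starting place and can be triggered again.
; Overlap starts a chain of Activated, Falling and Resetting events separated by delays, with physics simulation enabled for the drop.
; A timeline then lerps the platform from its fallen transform back to the one saved at BeginPlay.
; Material swaps and debug prints mark each state.
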(event `self.ReceiveBeginPlay`
  ; Begin Play
  (set `self.OriginalTransform` (`SceneComponent.K2_GetComponentToWorld` (`self.Platform`))) ; recording start location and rotation
  (`PrimitiveComponent.SetMaterial` (`self.Platform`) 0 "/Game/Materials/PlatformMaterials/MI_Platform_Ready.MI_Platform_Ready"))

(event `self.Box Trigger.OnComponentBeginOverlap`
  (params (OverlappedComponent :type "PrimitiveComponent Object Reference") (OtherActor :type "Actor Object Reference") (OtherComp :type "PrimitiveComponent Object Reference") (OtherBodyIndex :type Integer) (bFromSweep :type Boolean) (SweepResult :type "HitResult Structure (by ref)"))
  ;[0.08472 0.05365 0.15 0.5] Begin Overlap
  (`KismetSystemLibrary.PrintString` "Something ran into my trigger")
  (if (`self.isReady`)
    (cast `/Game/Blueprints/BP_Cust3rdPersonChar` OtherActor)
    (`self.Activated`)))

(event `Activated`
  ;[1 0.7 0 0] Activated
  (`KismetSystemLibrary.PrintString` "Activated")
  (`PrimitiveComponent.SetMaterial` (`self.Platform`) 0 "/Game/Materials/PlatformMaterials/MI_Platform_Activated.MI_Platform_Activated")
  (set `self.isReady` false)
  (`KismetSystemLibrary.Delay` (`self.fallDelayDuration`))
  (`self.Falling`))

(event `Falling`
  ;[0.15 0 0.01631 0.5] Falling
  (`KismetSystemLibrary.PrintString` "Falling")
  (`PrimitiveComponent.SetMaterial` (`self.Platform`) 0 "/Game/Materials/PlatformMaterials/MI_Platform_Falling.MI_Platform_Falling")
  (`PrimitiveComponent.SetSimulatePhysics` (`self.Platform`) true) ; Turns gravity on for the platform
  (`KismetSystemLibrary.Delay` (`self.fallDelayDuration`))
  (`self.Resetting`))

(event `Resetting`
  ;[0 0.15 0.003668 0.5] Resetting
  (`KismetSystemLibrary.PrintString` "Resetting")
  (set `self.FallenTransform` (`SceneComponent.K2_GetComponentToWorld` (`self.Platform`)))
  (`PrimitiveComponent.SetMaterial` (`self.Platform`) 0 "/Game/Materials/PlatformMaterials/MI_Platform_Resetting.MI_Platform_Resetting")
  (`PrimitiveComponent.SetSimulatePhysics` (`self.Platform`) false) ; Turns gravity off for the platform
  (bind (_direction _newtrack_0) (`Timeline|returntostart` :!via `PlayFromStart`)
    (:`Update`
      (bind (_returnvalue_location _returnvalue_rotation) (`KismetMathLibrary.BreakTransform` (`KismetMathLibrary.TLerp` (`self.FallenTransform`) (`self.OriginalTransform`) _newtrack_0)))
      (`SceneComponent.K2_SetWorldLocationAndRotation` (`self.Platform`) _returnvalue_location _returnvalue_rotation false false))
    (:`Finished`
      (set `self.isReady` true)
      (`PrimitiveComponent.SetMaterial` (`self.Platform`) 0 "/Game/Materials/PlatformMaterials/MI_Platform_Ready.MI_Platform_Ready"))))

(fn `UserConstructionScript`)