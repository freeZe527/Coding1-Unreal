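; BP_MovingPlat is a moving platform that travels between a Start and an End transform, starting automatically on BeginPlay.
; A timeline float track drives a transform lerp that sets the platform's world location and rotation on each update.
; Timeline event tracks swap the platform material to show a resetting look while moving and a ready look when stopped.
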(event `self.ReceiveBeginPlay`
  (bind (_direction _newtrack_0) (`Timeline|Timeline`)
    (:`Update`
      (bind (_returnvalue_location _returnvalue_rotation) (`KismetMathLibrary.BreakTransform` (`KismetMathLibrary.TLerp` (`SceneComponent.K2_GetComponentToWorld` (`self.Start`)) (`SceneComponent.K2_GetComponentToWorld` (`self.End`)) _newtrack_0)))
      (`SceneComponent.K2_SetWorldLocationAndRotation` (`self.Platform`) _returnvalue_location _returnvalue_rotation false false))
    (:`Moving`
      (`PrimitiveComponent.SetMaterial` (`self.Platform`) 0 "/Game/Materials/PlatformMaterials/MI_Platform_Resetting.MI_Platform_Resetting"))
    (:`Stopped`
      (`PrimitiveComponent.SetMaterial` (`self.Platform`) 0 "/Game/Materials/PlatformMaterials/MI_Platform_Ready.MI_Platform_Ready"))))

(fn `UserConstructionScript`)